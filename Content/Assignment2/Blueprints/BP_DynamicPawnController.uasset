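; BP_DynamicPawnController provides a debug readout of a pawn's attributes.
; Its DisplayAttributes event receives a pawn attribute asset and prints labeled health, speed and jump height strings, truncating speed to a whole number.
; BeginPlay, Tick and the construction script are empty, so output appears only when that event is called.
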(event EventBeginPlay)

(event EventTick
  (params (DeltaSeconds :type Float%20%28single-precision%29)))

(event EventDisplayAttributes
  (params (PawnAttributeAsset :type Pawn%20Attribute%20Asset%20Object%20Reference))
  (Development|PrintString (Utilities|String|Append "Health :" (Utilities|String|ToString(Integer) (Variables|/Script/Assignment2.PawnAttributeAsset|GetHealth PawnAttributeAsset))))
  (Development|PrintString (Utilities|String|Append "Speed :" (Utilities|String|ToString(Integer) (Math|Float|Truncate (Variables|/Script/Assignment2.PawnAttributeAsset|GetSpeed PawnAttributeAsset)))))
  (Development|PrintString (Utilities|String|Append "Jump Height :" (Utilities|String|ToString(Float) (Variables|/Script/Assignment2.PawnAttributeAsset|GetJumpHeight PawnAttributeAsset)))))

(fn ConstructionScript)